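; Player character Bob, who moves via Enhanced Input, turns toward a supplied target, shoots bullets and throws noisemakers.
; Left click and E play montages and spend limited ammo or noisemakers, with throw direction and clamped speed derived from the cursor hit point.
; DAMAGE reduces Health; death triggers an explosion and sounds, then reloads the level after a delay, which R forces through lethal damage.
; The input mapping context is re-added every Tick.
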(event Input|EnhancedActionEvents|EnhancedInputActionIA_movement
  (params (ActionValue :type Vector%202D%20Structure) (ElapsedSeconds :type Float%20%28double-precision%29) (TriggeredSeconds :type Float%20%28double-precision%29) (InputAction :type Input%20Action%20Object%20Reference :default "/Game/MyStuff/Character/IA_movement.IA_movement"))
  (bind _returnvalue (Pawn|GetControlRotation :!class /Script/Engine.Pawn))
  (:Triggered
    (if (not (<= (Variables|Default|GetHealth) 0.0))
      (Pawn|Input|AddMovementInput (Math|Vector|GetRightVector (Math|Rotator|MakeRotator (.roll _returnvalue) 0.0 (.yaw _returnvalue))) (.x ActionValue) false)
      (Pawn|Input|AddMovementInput (Math|Vector|GetForwardVector (Math|Rotator|MakeRotator 0.0 0.0 (.yaw (Pawn|GetControlRotation :!class /Script/Engine.Pawn)))) (.y ActionValue) false))))

(event EventDAMAGE
  (params (Amount :type Float%20%28double-precision%29))
  (Variables|Default|SetHealth (- (Variables|Default|GetHealth) Amount))
  (if (<= (Variables|Default|GetHealth) 0.0)
    (Utilities|FlowControl|DoOnce false
      (:Completed
        (bind _returnvalue (Game|GetCurrentLevelName true))
        (Effects|SpawnEmitteratLocation "/Game/StarterContent/Particles/P_Explosion.P_Explosion" (Transformation|GetActorLocation) "0, 0, 0" "3.000000,3.000000,3.000000")
        (Audio|PlaySound2D "/Game/StarterContent/Audio/Explosion01.Explosion01" 1.0 1.0 0.0 0 0)
        (Variables|Default|SetDead true)
        (Audio|PlaySound2D "/Game/MyStuff/Character/163442__under7dude__man-dying.163442__under7dude__man-dying" 1.0 1.0 0.0 0 0)
        (Utilities|FlowControl|Delay 2.0)
        (Game|OpenLevel(byName) (Utilities|String|StringToName _returnvalue))))))

(event EventBeginPlay
  (Variables|Default|SetRight%20Vec (.x (stale Input|EnhancedActionEvents|EnhancedInputActionIA_movement ActionValue)))
  (Variables|Default|SetForwardVec (.y (stale Input|EnhancedActionEvents|EnhancedInputActionIA_movement ActionValue))))

(event EventTick
  (params (DeltaSeconds :type Float%20%28single-precision%29))
  (bind _asplayer_controller (Utilities|Casting|CastToPlayerController (Pawn|GetController)))
  (Utilities|IsValid (PlayerController|LocalPlayerSubsystems|GetEnhancedInputLocalPlayerSubsystem _asplayer_controller)
    (:Is%20Valid
      (Input|AddMappingContext (PlayerController|LocalPlayerSubsystems|GetEnhancedInputLocalPlayerSubsystem _asplayer_controller) "/Game/MyStuff/Character/IMC_Bob.IMC_Bob" 0 "(bIgnoreAllPressedKeysUntilRelease=True,bForceImmediately=False)"))))

(event EventLookat
  (params (Target :type Vector :default "0, 0, 0"))
  (bind _returnvalue (Transformation|GetActorLocation))
  (Transformation|SetActorRotation (Math|Rotator|FindLookatRotation (Math|Vector|MakeVector (.x _returnvalue) (.y _returnvalue) 0.0) (Math|Vector|MakeVector (.x Target) (.y Target) 0.0))))

(event Input|MouseEvents|LeftMouseButton
  (params (Key :type Key%20Structure :default "None"))
  (bind _projectile_spawn (Variables|Default|GetProjectile_Spawn))
  (bind _returnvalue (Transformation|GetWorldTransform _projectile_spawn))
  (:Pressed
    (Animation|PlayAnimMontage "/Game/MyStuff/Character/Bob_Character/Animations/Bob_MM_Shoot.Bob_MM_Shoot" 1.0 "None")
    (if (> (Variables|Default|GetAmmo) 0)
      (Variables|Default|SetAmmo (- (Variables|Default|GetAmmo) 1))
      (Game|SpawnActorfromClass "/Game/MyStuff/Character/BP_bullet.BP_bullet_C" (Math|Transform|MakeTransform (.location _returnvalue) (.rotation _returnvalue) "0.600000,0.600000,0.600000") "AlwaysSpawn" 0 0))))

(event Input|KeyboardEvents|R
  (params (Key :type Key%20Structure :default "None"))
  (:Pressed
    (if (not (< (Variables|Default|GetHealth) 1.0))
      (CallFunction|DAMAGE 999.0))))

(event Input|KeyboardEvents|E
  (params (Key :type Key%20Structure :default "None"))
  (bind _returnvalue (Game|GetPlayerController 0))
  (bind _arrow1 (Variables|Default|GetArrow1))
  (bind _hitresult (Game|Player|GetHitResultUnderCursorbyChannel _returnvalue "TraceTypeQuery1" true))
  (bind _returnvalue_2 (Transformation|GetWorldLocation _arrow1))
  (bind _returnvalue_3 (Math|Rotator|FindLookatRotation _returnvalue_2 (.location _hitresult)))
  (bind _yaw (Math|Rotator|BreakRotator _returnvalue_3))
  (:Pressed
    (Animation|PlayAnimMontage "/Game/MyStuff/Character/Bob_Character/Animations/Bob_MM_Toss.Bob_MM_Toss" 1.0 "None")
    (if (> (Variables|Default|GetNoiseMakers) 0)
      (Variables|Default|SetThrowing true)
      (bind _returnvalue_4 (Game|SpawnActorfromClass "/Game/MyStuff/Character/Botte/NoiseMaker.NoiseMaker_C" (Math|Transform|MakeTransform (Transformation|GetWorldLocation (Variables|Default|GetArrow1)) (Math|Rotator|MakeRotator 0.0 0.0 _yaw) "40.000000,40.000000,40.000000") "Undefined" 0 0))
      (Variables|Default|SetNoiseMakers (- (Variables|Default|GetNoiseMakers) 1))
      (Variables|/Script/Engine.MovementComponent|SetVelocity (Variables|/Game/MyStuff/Character/Botte/NoiseMaker.NoiseMaker_C|GetProjectileMovement _returnvalue_4) (Math|Vector|RotateVector (Math|Vector|MakeVector (Math|Float|Clamp(Float) (* (Math|Vector|Distance(Vector) (.location _hitresult) _returnvalue_2) 1.75) 3.5e+02 1.5e+03) 0.0 0.0) (Math|Rotator|MakeRotator 0.0 0.0 _yaw)))
      (Variables|Default|SetThrowing false))))

(fn ConstructionScript)