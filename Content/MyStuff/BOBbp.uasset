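; BOBbp is the player-controlled shooter Blueprint for Bob, with movement, health and ammo.
; Tick re-adds the IMC_Bob input mapping every frame; movement follows control rotation while health remains, and a Lookat event turns the actor toward a target.
; Left click spends ammo to spawn a bullet at ProjectileSpawn.
; DAMAGE lowers health, and death triggers an explosion, then loads MORTEMFIEND after a delay.
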(event Input|EnhancedActionEvents|EnhancedInputActionIA_movement
  (params (ActionValue :type Vector%202D%20Structure) (ElapsedSeconds :type Float%20%28double-precision%29) (TriggeredSeconds :type Float%20%28double-precision%29) (InputAction :type Input%20Action%20Object%20Reference :default "/Game/MyStuff/Character/IA_movement.IA_movement"))
  (bind _returnvalue (Pawn|GetControlRotation :!class /Script/Engine.Pawn))
  (:Triggered
    (if (not (<= (Variables|Default|GetHealth) 0.0))
      (Pawn|Input|AddMovementInput (Math|Vector|GetRightVector (Math|Rotator|MakeRotator (.roll _returnvalue) 0.0 (.yaw _returnvalue))) (.x ActionValue) false)
      (Pawn|Input|AddMovementInput (Math|Vector|GetForwardVector (Math|Rotator|MakeRotator 0.0 0.0 (.yaw (Pawn|GetControlRotation :!class /Script/Engine.Pawn)))) (.y ActionValue) false))))

(event EventDAMAGE
  (params (Amount :type Float%20%28double-precision%29))
  (Variables|Default|SetHealth (- (Variables|Default|GetHealth) Amount))
  (if (<= (Variables|Default|GetHealth) 0.0)
    (Effects|SpawnEmitteratLocation "/Game/StarterContent/Particles/P_Explosion.P_Explosion" (Transformation|GetActorLocation) "0, 0, 0" "3.000000,3.000000,3.000000")
    (Audio|PlaySound2D "/Game/StarterContent/Audio/Explosion01.Explosion01" 1.0 1.0 0.0 0 0)
    (Utilities|FlowControl|Delay 1.0)
    (Game|OpenLevel(byName) "MORTEMFIEND")))

(event EventDestroyed)

(event EventTick
  (params (DeltaSeconds :type Float%20%28single-precision%29))
  (bind _asplayer_controller (Utilities|Casting|CastToPlayerController (Pawn|GetController)))
  (Utilities|IsValid (PlayerController|LocalPlayerSubsystems|GetEnhancedInputLocalPlayerSubsystem _asplayer_controller)
    (:Is%20Valid
      (Input|AddMappingContext (PlayerController|LocalPlayerSubsystems|GetEnhancedInputLocalPlayerSubsystem _asplayer_controller) "/Game/MyStuff/Character/IMC_Bob.IMC_Bob" 0 "(bIgnoreAllPressedKeysUntilRelease=True,bForceImmediately=False)"))))

(event EventLookat
  (params (Target :type Vector :default "0, 0, 0"))
  (bind _returnvalue (Transformation|GetActorLocation))
  (Transformation|SetActorRotation (Math|Rotator|FindLookatRotation (Math|Vector|MakeVector (.x _returnvalue) (.y _returnvalue) 0.0) (Math|Vector|MakeVector (.x Target) (.y Target) 0.0))))

(event Input|MouseEvents|LeftMouseButton
  (params (Key :type Key%20Structure :default "None"))
  (bind _projectile_spawn (Variables|Default|GetProjectile_Spawn))
  (bind _returnvalue (Transformation|GetWorldTransform _projectile_spawn))
  (:Pressed
    (if (> (Variables|Default|GetAmmo) 0)
      (Variables|Default|SetAmmo (- (Variables|Default|GetAmmo) 1))
      (Development|PrintString (Utilities|String|ToString(Integer) (Variables|Default|GetAmmo)))
      (Game|SpawnActorfromClass "/Game/MyStuff/BP_bullet.BP_bullet_C" (Math|Transform|MakeTransform (.location _returnvalue) (.rotation _returnvalue) "0.400000,0.400000,0.400000") "AlwaysSpawn" 0 0))))

(fn ConstructionScript)